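; HUD Blueprint for Grimsby, a werewolf-themed game, that creates the main widget and holds state for notifications and end screens.
; ShowFullMoonHUD and ShowHumanityChange reveal notices and set flags, which Tick consumes to hide them after short delays.
; Tick also polls Health and Humanity, pausing the game with a cursor and ending text for death (varied by Kills), a cured beast, or total humanity loss.
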(event EventBeginPlay
  (bind _returnvalue (UserInterface|CreateWidget "/Game/Blueprints/Grimsby_Widget.Grimsby_Widget_C"))
  (UserInterface|Viewport|AddtoViewport _returnvalue 0))

(event Collision|EventActorBeginOverlap
  (params (OtherActor :type Actor%20Object%20Reference)))

(event EventTick
  (params (DeltaSeconds :type Float%20%28single-precision%29))
  (Utilities|FlowControl|Sequence
    (:then_0
      (if (Variables|Default|GetfullMoonBool)
        (Variables|Default|SetfullMoonBool false)
        (Utilities|FlowControl|Delay 2.0)
        (Variables|Default|SetfullMoon "Hidden")))
    (:then_1
      (if (Variables|Default|GethumanityChangeBool)
        (Variables|Default|SethumanityChangeBool false)
        (Utilities|FlowControl|Delay 1.0)
        (Variables|Default|SethumanityChangeState "Hidden")))
    (:then_2
      (if (<= (Variables|Default|GetHealth) 0)
        (Game|SetGamePaused true)
        (Variables|/Script/Engine.PlayerController|SetbShowMouseCursor (Game|GetPlayerController 0) true)
        (Variables|Default|SetendScreenTitle "You Died!")
        (if (> (Variables|Default|GetKills) 0)
          (Variables|Default|SetendScreenContent (Utilities|String|MakeLiteralString "Although you have died due to full moon exposure, you did not die alone. Take comfort in knowing you died with your other half and that the lives of the people you've destroyed were the only legacy you two left behind."))
          (Variables|Default|SetendScreenVisibility "Visible")
          (else
            (Variables|Default|SetendScreenContent (Utilities|String|MakeLiteralString "Although you have died due to full moon exposure, you did not die alone. Take comfort in knowing you died with your other half - who - while you were not able to defeat, stood up to, not once killing a single soul."))
            (Variables|Default|SetendScreenVisibility "Visible")))
        (elif (>= (Variables|Default|GetHumanity) 1e+03)
          (Game|SetGamePaused true)
          (Variables|/Script/Engine.PlayerController|SetbShowMouseCursor (Game|GetPlayerController 0) true)
          (Variables|Default|SetendScreenTitle "The Beast Has Vanished!")
          (Variables|Default|SetendScreenContent "A great weight has been lifted... I can feel it. The moon no longer beckons, nor does the monster inside me. But why don't I feel happy? Relieved? Content? Why do I feel ... empty.")
          (Variables|Default|SetendScreenVisibility "Visible")
          (elif (<= (Variables|Default|GetHumanity) 0.0)
            (Game|SetGamePaused true)
            (Variables|/Script/Engine.PlayerController|SetbShowMouseCursor (Game|GetPlayerController 0) true)
            (Variables|Default|SetendScreenTitle "Only The Beast Remains!")
            (Variables|Default|SetendScreenContent "With not a scrape of humanity to your name, you die, leaving only the monster behind to reek havoc upon the citizens of Grimsby... They didn't stand a chance.")
            (Variables|Default|SetendScreenVisibility "Visible")))))))

(fn ConstructionScript)

(fn ShowFullMoonHUD
  (Variables|Default|SetfullMoon "Visible")
  (Variables|Default|SetfullMoonBool true))

(fn ShowHumanityChange
  (params (humanity :type String))
  (Variables|Default|SethumanityChangeState "Visible")
  (Variables|Default|SethumanityChangeBool true)
  (Variables|Default|SethumanityChangeVal humanity))